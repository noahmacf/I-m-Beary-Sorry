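; Paper2D flipbook character that moves on the world X/Y plane from axis input, with Left Shift switching between walk and run fly speeds.
; Each tick, SetDirection stores the input-based facing and picks a directional idle, walk or run flipbook from velocity and run state.
; CalculateZ then traces downward and sets actor height to the impact point plus DistanceZ.
; The construction script tilts the sprite to match the spring arm's pitch.
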(event EventBeginPlay)

(event EventTick
  (params (DeltaSeconds :type Float%20%28single-precision%29))
  (CallFunction|SetDirection)
  (CallFunction|CalculateZ))

(event Input|AxisEvents|InputAxisXAxis
  (params (AxisValue :type Float%20%28single-precision%29))
  (Pawn|Input|AddMovementInput "0,1.000000, 0" AxisValue false))

(event Input|AxisEvents|InputAxisYAxis
  (params (AxisValue :type Float%20%28single-precision%29))
  (Pawn|Input|AddMovementInput "-1.000000, 0, 0" AxisValue false))

(event Input|KeyboardEvents|LeftShift
  (params (Key :type Key%20Structure :default "None"))
  (bind _charactermovement (Variables|Character|GetCharacterMovement))
  (:Pressed
    (Variables|/Script/Engine.CharacterMovementComponent|SetMaxFlySpeed _charactermovement 7.5e+02)
    (Variables|Default|SetisRunning true))
  (:Released
    (Variables|/Script/Engine.CharacterMovementComponent|SetMaxFlySpeed _charactermovement 3e+02)
    (Variables|Default|SetisRunning false)))

(fn ConstructionScript
  (Transformation|SetWorldRotation (Variables|Default|GetSprite) (Math|Rotator|MakeRotator (.pitch (Transformation|GetWorldRotation (Variables|Default|GetSpringArm))) 0.0 -9e+01) false false))

(fn SetDirection
  (bind _returnvalue (Transformation|GetVelocity))
  (bind _sprite (Variables|Default|GetSprite))
  (bind _returnvalue_2 (Math|Vector|VectorLength _returnvalue))
  (bind _returnvalue_3 (> _returnvalue_2 0.0))
  (if (or (!= (Input|AxisValues|GetXAxis) 0.0) (!= (Input|AxisValues|GetYAxis) 0.0))
    (Variables|Default|SetDirection (select (< (Input|AxisValues|GetYAxis) 0.0) "NewEnumerator0" (select (> (Input|AxisValues|GetYAxis) 0.0) "NewEnumerator1" (select (> (Input|AxisValues|GetXAxis) 0.0) "NewEnumerator2" "NewEnumerator3"))))
    (if (Variables|Default|GetisRunning)
      (Sprite|SetFlipbook _sprite (select _returnvalue_3 (Utilities|Select :Index (Variables|Default|GetDirection) :NewEnumerator0 "/Game/Blueprints/FB_Run_Down.FB_Run_Down" :NewEnumerator1 "/Game/Blueprints/FB_Run_Up.FB_Run_Up" :NewEnumerator2 "/Game/Blueprints/FB_Run_Left.FB_Run_Left" :NewEnumerator3 "/Game/Blueprints/FB_Run_Right.FB_Run_Right") (Utilities|Select :Index (Variables|Default|GetDirection) :NewEnumerator0 "/Game/Blueprints/FB_Idle_Down.FB_Idle_Down" :NewEnumerator1 "/Game/Blueprints/FB_Idle_Up.FB_Idle_Up" :NewEnumerator2 "/Game/Blueprints/FB_Idle_Left.FB_Idle_Left" :NewEnumerator3 "/Game/Blueprints/FB_Idle_Right.FB_Idle_Right")))
      (else
        (Sprite|SetFlipbook _sprite (select _returnvalue_3 (Utilities|Select :Index (Variables|Default|GetDirection) :NewEnumerator0 "/Game/Blueprints/FB_Walk_Down.FB_Walk_Down" :NewEnumerator1 "/Game/Blueprints/FB_Walk_Up.FB_Walk_Up" :NewEnumerator2 "/Game/Blueprints/FB_Walk_Left.FB_Walk_Left" :NewEnumerator3 "/Game/Blueprints/FB_Walk_Right.FB_Walk_Right") (Utilities|Select :Index (Variables|Default|GetDirection) :NewEnumerator0 "/Game/Blueprints/FB_Idle_Down.FB_Idle_Down" :NewEnumerator1 "/Game/Blueprints/FB_Idle_Up.FB_Idle_Up" :NewEnumerator2 "/Game/Blueprints/FB_Idle_Left.FB_Idle_Left" :NewEnumerator3 "/Game/Blueprints/FB_Idle_Right.FB_Idle_Right")) :!label _label)))
    (else
      (goto _label))))

(fn CalculateZ
  (bind _returnvalue (Transformation|GetActorLocation))
  (bind _returnvalue_2 (Transformation|GetActorLocation))
  (bind _outhit (Collision|LineTraceByChannel (Transformation|GetActorLocation) (Math|Vector|MakeVector (.x _returnvalue) (.y _returnvalue) (- (.z _returnvalue) 2e+02)) "TraceTypeQuery1" false 0 "None"))
  (Transformation|SetActorLocation (Math|Vector|MakeVector (.x _returnvalue_2) (.y _returnvalue_2) (+ (.z (.ImpactPoint (Collision|BreakHitResult _outhit))) (Variables|Default|GetDistanceZ))) false false))